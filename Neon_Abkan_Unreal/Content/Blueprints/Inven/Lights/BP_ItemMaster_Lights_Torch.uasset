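; Torch light item Blueprint in the inventory's Lights set, built around a SpotLight.
; BeginPlay caches the SpotLight's intensity in an Intensity variable, and the construction script only calls the parent's.
; An unconnected node chain would step the intensity down, print it and apply it to the light, but it never runs, and Tick is empty.
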(event EventTick
  (params (DeltaSeconds :type Float%20%28single-precision%29)))

(event EventBeginPlay
  (Variables|Default|SetIntensity (Variables|/Script/Engine.LightComponentBase|GetIntensity (Variables|Default|GetSpotLight))))

(fn ConstructionScript
  (|CallParentFunction))