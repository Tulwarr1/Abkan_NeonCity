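; ClassRooms is a classroom Blueprint that randomizes its resource pickups when play begins.
; It loops over every component sharing the class of the placed wood resource component, which serve as child-actor slots.
; A random roll per slot swaps the child actor class to nails, metal, wire or wood, or destroys the component to leave that spot empty.
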(event EventBeginPlay
  (bind _bp_itemmaster__resources_wood (Variables|Default|GetBP_ItemMaster__Resources_Wood))
  (bind _returnvalue (Utilities|GetClass _bp_itemmaster__resources_wood))
  (bind _returnvalue_2 (Actor|GetComponentsByClass _returnvalue))
  (for (_ _array_index) _returnvalue_2
    (bind _output_get (Variables|Default|SetRanID (Math|Random|RandomIntegerinRange 0 4)))
    (switch int _output_get
      (:0
        (ChildActorComponent|SetChildActorClass (Utilities|Array|Get(acopy) _returnvalue_2 _array_index) "/Game/Blueprints/Inven/Resources/BP_ItemMaster__Resources_Nails.BP_ItemMaster__Resources_Nails_C"))
      (:1
        (ChildActorComponent|SetChildActorClass (Utilities|Array|Get(acopy) _returnvalue_2 _array_index) "/Game/Blueprints/Inven/Resources/BP_ItemMaster__Resources_Metal.BP_ItemMaster__Resources_Metal_C"))
      (:2
        (ChildActorComponent|SetChildActorClass (Utilities|Array|Get(acopy) _returnvalue_2 _array_index) "/Game/Blueprints/Inven/Resources/BP_ItemMaster__Resources_Wire.BP_ItemMaster__Resources_Wire_C"))
      (:3
        (ChildActorComponent|SetChildActorClass (Utilities|Array|Get(acopy) _returnvalue_2 _array_index) "/Game/Blueprints/Inven/Resources/BP_ItemMaster__Resources_Wood.BP_ItemMaster__Resources_Wood_C"))
      (:4
        (Components|DestroyComponent (Utilities|Array|Get(acopy) _returnvalue_2 _array_index))))))

(fn ConstructionScript)