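; Blue_Projectile is a projectile that relocates the Blue_Portato when it hits something.
; On Hit it finds and destroys the first existing Blue_Portato and destroys itself.
; It then spawns a new Blue_Portato pulled back from the projectile's location against its forward vector, always spawning regardless of collision.
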(event EventBeginPlay)

(event EventActorBeginOverlap
  (params (OtherActor :type Actor%20Object%20Reference)))

(event EventTick
  (params (DeltaSeconds :type Float%20%28single-precision%29)))

(event Collision|EventHit
  (params (MyComp :type Primitive%20Component%20Object%20Reference) (Other :type Actor%20Object%20Reference) (OtherComp :type Primitive%20Component%20Object%20Reference) (bSelfMoved :type Boolean) (HitLocation :type Vector :default "0, 0, 0") (HitNormal :type Vector :default "0, 0, 0") (NormalImpulse :type Vector :default "0, 0, 0") (Hit :type Hit%20Result%20Structure%20%28by%20ref%29))
  (bind _outactors (Actor|GetAllActorsOfClass "/Game/Blueprints/Portatoes/Blue_Portato.Blue_Portato_C"))
  (Actor|DestroyActor (Utilities|Array|Get(acopy) _outactors))
  (Actor|DestroyActor)
  (Game|SpawnActorfromClass "/Game/Blueprints/Portatoes/Blue_Portato.Blue_Portato_C" (Math|Conversions|ToTransform(Vector) (+ (* (Math|Vector|GetForwardVector (Transformation|GetActorRotation)) -100) (Transformation|GetActorLocation))) "AlwaysSpawn" 0 0))

(fn ConstructionScript)