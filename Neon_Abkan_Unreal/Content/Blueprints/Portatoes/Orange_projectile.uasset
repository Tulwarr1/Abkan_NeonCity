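; Orange portal-style projectile that places an Orange_Portato where it hits.
; On hit, it destroys the first existing Orange_Portato found in the level and then itself.
; It then spawns a replacement 100 units back along its forward vector from its location, passing only that position into the spawn transform.
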(event Collision|EventHit
  (params (MyComp :type Primitive%20Component%20Object%20Reference) (Other :type Actor%20Object%20Reference) (OtherComp :type Primitive%20Component%20Object%20Reference) (bSelfMoved :type Boolean) (HitLocation :type Vector :default "0, 0, 0") (HitNormal :type Vector :default "0, 0, 0") (NormalImpulse :type Vector :default "0, 0, 0") (Hit :type Hit%20Result%20Structure%20%28by%20ref%29))
  (bind _outactors (Actor|GetAllActorsOfClass "/Game/Blueprints/Portatoes/Orange_Portato.Orange_Portato_C"))
  (Actor|DestroyActor (Utilities|Array|Get(acopy) _outactors))
  (Actor|DestroyActor)
  (Game|SpawnActorfromClass "/Game/Blueprints/Portatoes/Orange_Portato.Orange_Portato_C" (Math|Conversions|ToTransform(Vector) (+ (* (Math|Vector|GetForwardVector (Transformation|GetActorRotation)) -100) (Transformation|GetActorLocation))) "Undefined" 0 0))

(fn ConstructionScript)