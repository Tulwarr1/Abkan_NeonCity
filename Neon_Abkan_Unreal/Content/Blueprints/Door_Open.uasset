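; Double-door Blueprint that lets the player open and close two meshes with the E key.
; Overlapping the T_OpenDoor trigger enables input from player 0, and leaving it disables input, without checking which actor overlapped.
; A FlipFlop on E plays or reverses a timeline that yaws the meshes in opposite directions, setting absolute world rotation.
; The T_CloseDoor end-overlap event is empty.
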(event OnComponentBeginOverlap(T_OpenDoor)
  (params (OtherActor :type Actor%20Object%20Reference) (OtherComp :type Primitive%20Component%20Object%20Reference) (OtherBodyIndex :type Integer) (bFromSweep :type Boolean) (SweepResult :type Hit%20Result%20Structure%20%28by%20ref%29))
  (Input|EnableInput (Game|GetPlayerController 0)))

(event OnComponentEndOverlap(T_OpenDoor)
  (params (OtherActor :type Actor%20Object%20Reference) (OtherComp :type Primitive%20Component%20Object%20Reference) (OtherBodyIndex :type Integer))
  (Input|DisableInput (Game|GetPlayerController 0)))

(event OnComponentEndOverlap(T_CloseDoor)
  (params (OtherActor :type Actor%20Object%20Reference) (OtherComp :type Primitive%20Component%20Object%20Reference) (OtherBodyIndex :type Integer)))

(event Input|KeyboardEvents|E
  (params (Key :type Key%20Structure :default "AnyKey"))
  (:Pressed
    (Utilities|FlowControl|FlipFlop
      (:A
        (bind _doorrot (Timeline|Timeline_0 Play)
          (:Update
            (Transformation|SetWorldRotation (Variables|Default|GetStaticMesh) (Math|Rotator|MakeRotator 0.0 0.0 _doorrot) false false)
            (Transformation|SetWorldRotation (Variables|Default|GetStaticMesh1) (* (Math|Rotator|MakeRotator 0.0 0.0 _doorrot) -1.0) false false))))
      (:B
        (Timeline|Timeline_0 Reverse)))))

(fn ConstructionScript)