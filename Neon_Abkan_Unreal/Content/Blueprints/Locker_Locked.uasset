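; Interactive locker that the player opens and closes with E, or that plays a separate locked door motion when CanOpen is false.
; Overlapping its Box enables input on player controller 0, and leaving disables it.
; When openable, a FlipFlop plays or reverses the door timeline; when locked, a second timeline replays, guarded by a DoOnce until finished.
; Both timelines set the door's yaw in world space.
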(event OnComponentBeginOverlap(Box)
  (params (OtherActor :type Actor%20Object%20Reference) (OtherComp :type Primitive%20Component%20Object%20Reference) (OtherBodyIndex :type Integer) (bFromSweep :type Boolean) (SweepResult :type Hit%20Result%20Structure%20%28by%20ref%29))
  (Input|EnableInput (Game|GetPlayerController 0)))

(event OnComponentEndOverlap(Box)
  (params (OtherActor :type Actor%20Object%20Reference) (OtherComp :type Primitive%20Component%20Object%20Reference) (OtherBodyIndex :type Integer))
  (Input|DisableInput (Game|GetPlayerController 0)))

(event Input|KeyboardEvents|E
  (params (Key :type Key%20Structure :default "AnyKey"))
  (:Pressed
    (if (Variables|Default|GetCanOpen)
      ;[1 1 1] Open
      (Utilities|FlowControl|FlipFlop
        (:A
          (bind _doorrot (Timeline|Timeline_0 Play)
            (:Update
              (Transformation|SetWorldRotation (Variables|Default|GetLocker_02_door) (Math|Rotator|MakeRotator 0.0 0.0 _doorrot) false false))))
        (:B
          (Timeline|Timeline_0 Reverse)))
      (else
        ;[1 1 1] Locked
        (Utilities|FlowControl|DoOnce false :!label _label
          (:Completed
            (bind _doorrot_2 (Timeline|Timeline_1 PlayFromStart)
              (:Update
                (Transformation|SetWorldRotation (Variables|Default|GetLocker_02_door) (Math|Rotator|MakeRotator 0.0 0.0 _doorrot_2) false false))
              (:Finished
                (goto _label Reset)))))))))

(fn ConstructionScript)