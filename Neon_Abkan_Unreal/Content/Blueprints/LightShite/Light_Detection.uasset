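; Light detection Blueprint with Dim and Bright trigger components that drives the player's Sanity from light exposure.
; Overlaps set light flags on Player_01; each Tick raises sanity in light, faster in Bright, and drains it in darkness, without delta-time scaling.
; An active torch sets the dim flag, which only a Dim end-overlap clears.
; At 80 or below, monster growls repeat at random intervals; zero sets GameOver.
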(event OnComponentBeginOverlap(Dim)
  (params (OtherActor :type Actor%20Object%20Reference) (OtherComp :type Primitive%20Component%20Object%20Reference) (OtherBodyIndex :type Integer) (bFromSweep :type Boolean) (SweepResult :type Hit%20Result%20Structure%20%28by%20ref%29))
  (bind _char (Variables|Default|GetChar))
  ;[1 1 1] Light Detection
  (Variables|Default|SetIs_In_Dim true)
  (Variables|/Game/Blueprints/Player_01.Player_01_C|SetInLight _char true)
  (Variables|/Game/Blueprints/Player_01.Player_01_C|SetLightValue _char 1))

(event OnComponentBeginOverlap(Bright)
  (params (OtherActor :type Actor%20Object%20Reference) (OtherComp :type Primitive%20Component%20Object%20Reference) (OtherBodyIndex :type Integer) (bFromSweep :type Boolean) (SweepResult :type Hit%20Result%20Structure%20%28by%20ref%29))
  ;[1 1 1] Light Detection
  (Variables|Default|SetIs_In_Bright true))

(event OnComponentEndOverlap(Dim)
  (params (OtherActor :type Actor%20Object%20Reference) (OtherComp :type Primitive%20Component%20Object%20Reference) (OtherBodyIndex :type Integer))
  (bind _char (Variables|Default|GetChar))
  ;[1 1 1] Light Detection
  (Variables|Default|SetIs_In_Dim false)
  (Variables|/Game/Blueprints/Player_01.Player_01_C|SetInLight _char false)
  (Variables|/Game/Blueprints/Player_01.Player_01_C|SetLightValue _char 0))

(event OnComponentEndOverlap(Bright)
  (params (OtherActor :type Actor%20Object%20Reference) (OtherComp :type Primitive%20Component%20Object%20Reference) (OtherBodyIndex :type Integer))
  ;[1 1 1] Light Detection
  (Variables|Default|SetIs_In_Bright false))

(event EventBeginPlay
  ;[1 1 1] Sets Shit
  (Variables|Default|SetLD_Sanity 1e+02)
  (bind _asplayer_01 (Utilities|Casting|CastToPlayer_01 (Game|GetPlayerCharacter 0)))
  (Variables|Default|SetChar _asplayer_01))

(event EventTick
  (params (DeltaSeconds :type Float%20%28single-precision%29))
  (bind _char (Variables|Default|GetChar))
  (Variables|/Game/Blueprints/Player_01.Player_01_C|SetSanity _char (Variables|Default|GetLD_Sanity))
  (if (Variables|/Game/Blueprints/Player_01.Player_01_C|GetPlayerTorch _char)
    (Variables|Default|SetIs_In_Dim true))
  (if (> (Variables|/Game/Blueprints/Player_01.Player_01_C|GetLightValue _char) 0)
    (if (Variables|Default|GetIs_In_Bright) :!label _label
      ;[1 1 1] Bright Light Incress
      (Variables|Default|SetLD_Sanity (Math|Float|Clamp(Float) (+ (Variables|Default|GetLD_Sanity) 0.05) 0.0 1e+02))
      (else
        ;[1 1 1] Bright Light Incress
        (Variables|Default|SetLD_Sanity (Math|Float|Clamp(Float) (+ (Variables|Default|GetLD_Sanity) 0.025) 0.0 1e+02))))
    (elif (Variables|Default|GetIs_In_Dim)
      (goto _label)
      (else
        ;[1 1 1] Light Decress
        (Variables|Default|SetLD_Sanity (Math|Float|Clamp(Float) (- (Variables|Default|GetLD_Sanity) 0.025) 0.0 1e+02)))))
  (if (<= (Variables|Default|GetLD_Sanity) 0.0)
    (Variables|Default|SetGameOver true)
    (elif (<= (Variables|Default|GetLD_Sanity) 8e+01)
      (Utilities|FlowControl|DoOnce false :!label _label_2
        (:Completed
          (Audio|PlaySoundatLocation "/Game/Sounds/Monster_Growl-SoundBible_com-344645592.Monster_Growl-SoundBible_com-344645592" (Transformation|GetWorldLocation (Variables|/Script/Engine.Character|GetCapsuleComponent (Variables|Default|GetChar))) "0, 0, 0" 1.0 1.0 0.5)
          (Utilities|FlowControl|Delay (Math|Random|RandomFloatinRange 8.0 2e+01))
          (goto _label_2 Reset))))))

(fn ConstructionScript)